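; Enemy spawner for an ant game, built to create generations of evolving enemies, though its events are empty and the spawn logic is disconnected.
; The unwired logic feeds player colony counts to CreateFirstGeneration, or adds previous enemies' combat stats for Evolve.
; It spawns one CharBP_Enemy per player ant, giving each AI controller four behavior weights from the flat output array.
; Only the first-generation path binds the death delegate, whose handler is empty.
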(event `self.ReceiveBeginPlay`)

(event `self.ReceiveActorBeginOverlap`
  (params (OtherActor :type "Actor Object Reference")))

(event `self.ReceiveTick`
  (params (DeltaSeconds :type "Float (single-precision)")))

(event `OnDiedDelegate_Event_0`
  (params (DeadCharacter :type "BaseCharacter Object Reference")))

(event `SpawnFirstEnemies`
  (params (Location :type "Vector Structure"))
  ;[1 1 1] Spawn first enemies
)

(event `SpawnEnemies`
  ;[1 1 1] Evolve enemies to spawn next generation
)

(fn `UserConstructionScript`)