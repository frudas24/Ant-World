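; Spawner for the colony's five ant types (Builder, Collector, Processor, Cleaner, Guard), creating the starting ants and ones bought through PlCtrl_TCC events.
; Each spawn gets an AI controller, joins the Ants array and HUD, and updates the player controller's counts.
; Death delegates undo this, tally deaths and call GameOver when no ants remain and CanGameOver is set.
; Retreat withdraws every ant, then after a delay clears under-attack flags and EnemiesLeft.
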(event `BoughtBuilder_Event_0`
  (`self.AddNewBuilder`))

(event `BoughtCollector_Event_0`
  (`self.AddNewCollector`))

(event `BoughtProcessor_Event_0`
  (`self.AddNewProcessor`))

(event `self.ReceiveBeginPlay`
  (bind _aspl_ctrl_tcc (cast `/Game/Blueprints/PlCtrl_TCC` (`GameplayStatics.GetPlayerController` 0)))
  (add `/Game/Blueprints/PlCtrl_TCC.GameStarted` _aspl_ctrl_tcc (delegate `GameStarted`))
  (add `/Game/Blueprints/PlCtrl_TCC.BoughtBuilder` _aspl_ctrl_tcc (delegate `BoughtBuilder_Event_0`))
  (add `/Game/Blueprints/PlCtrl_TCC.BoughtCleaner` _aspl_ctrl_tcc (delegate `BoughtCleaner_Event_0`))
  (add `/Game/Blueprints/PlCtrl_TCC.BoughtCollector` _aspl_ctrl_tcc (delegate `BoughtCollector_Event_0`))
  (add `/Game/Blueprints/PlCtrl_TCC.BoughtGuard` _aspl_ctrl_tcc (delegate `BoughtGuard_Event_0`))
  (add `/Game/Blueprints/PlCtrl_TCC.BoughtProcessor` _aspl_ctrl_tcc (delegate `BoughtProcessor_Event_0`)))

(event `BoughtCleaner_Event_0`
  (`self.AddNewCleaner`))

(event `BoughtGuard_Event_0`
  (`self.AddNewGuard`))

(event `GameStarted`
  (params (Level :type Integer))
  ;[1 1 1] Spanw first ants
)

(event `SpawnFirstAnts`
  (params (Builder :type Integer) (Collector :type Integer) (Processor :type Integer) (Cleaner :type Integer) (Guard :type Integer) (CanGameOver :type Boolean))
  ;[1 1 1] Spanw first ants
  (for _ (range 1 (+ Builder 1))
    (`self.AddNewBuilder`))
  (for _ (range 1 (+ Collector 1))
    (`self.AddNewCollector`))
  (for _ (range 1 (+ Processor 1))
    (`self.AddNewProcessor`))
  (for _ (range 1 (+ Cleaner 1))
    (`self.AddNewCleaner`))
  (for _ (range 1 (+ Guard 1))
    (`self.AddNewGuard`))
  (set `self.CanGameOver` CanGameOver))

(event `AddNewCollector`
  (bind _aspl_ctrl_tcc (cast `/Game/Blueprints/PlCtrl_TCC` (`GameplayStatics.GetPlayerController` 0)))
  (bind _returnvalue (`|SpawnActorFromClass` "/Game/Blueprints/Characters/CharacterBlueprints/Ants/CharBP_Collector.CharBP_Collector_C" (`KismetMathLibrary.MakeTransform` (950.0 0.0 30.0)) "AlwaysSpawn" "OverrideRootScale"))
  (`Pawn.SpawnDefaultController` _returnvalue)
  (bind _returnvalue_2 (`KismetArrayLibrary.Array_Add` (`self.Ants`) _returnvalue))
  (bind _output_get (set `TCCPlayerController.CollectorQtt` (+ (stale _output_get) 1) _aspl_ctrl_tcc))
  (bind _output_get_2 (set `TCCPlayerController.AntsQtt` (+ (stale _output_get_2) 1) _aspl_ctrl_tcc))
  (add `BaseCharacter.OnDiedDelegate` _returnvalue (delegate `OnDiedDelegate_Event_0`))
  (bind _index (`/Game/HUD/Wid_InGame.AddNewAnt` (`/Game/Blueprints/PlCtrl_TCC.InGameHud` _aspl_ctrl_tcc) _returnvalue))
  (`KismetArrayLibrary.Array_Set` (`self.WidgetIndex`) _returnvalue_2 _index true))

(event `OnDiedDelegate_Event_0`
  (params (DeadCharacter :type "BaseCharacter Object Reference"))
  (bind _ants (`self.Ants`))
  (bind _returnvalue (`KismetArrayLibrary.Array_Find` _ants DeadCharacter))
  (bind _aspl_ctrl_tcc (cast `/Game/Blueprints/PlCtrl_TCC` (`GameplayStatics.GetPlayerController` 0)))
  (bind _output_get (set `TCCPlayerController.CollectorQtt` (- (stale _output_get) 1) _aspl_ctrl_tcc))
  (bind _output_get_2 (set `TCCPlayerController.AntsQtt` (- (stale _output_get_2) 1) _aspl_ctrl_tcc))
  (`/Game/HUD/Wid_InGame.RemoveAnt` (`/Game/Blueprints/PlCtrl_TCC.InGameHud` _aspl_ctrl_tcc) _returnvalue)
  (`KismetArrayLibrary.Array_Remove` (`self.WidgetIndex`) _returnvalue)
  (`KismetArrayLibrary.Array_RemoveItem` _ants DeadCharacter)
  (bind _output_get_3 (set `TCCPlayerController.CollectorDead` (+ (stale _output_get_3) 1) _aspl_ctrl_tcc))
  (if (and (<= (`TCCPlayerController.AntsQtt` _aspl_ctrl_tcc) 0) (`self.CanGameOver`))
    (`/Game/Blueprints/PlCtrl_TCC.GameOver` _aspl_ctrl_tcc)))

(event `AddNewBuilder`
  (bind _aspl_ctrl_tcc (cast `/Game/Blueprints/PlCtrl_TCC` (`GameplayStatics.GetPlayerController` 0)))
  (bind _returnvalue (`|SpawnActorFromClass` "/Game/Blueprints/Characters/CharacterBlueprints/Ants/CharBP_Builder.CharBP_Builder_C" (`KismetMathLibrary.MakeTransform` (950.0 0.0 30.0)) "AlwaysSpawn" "OverrideRootScale"))
  (`Pawn.SpawnDefaultController` _returnvalue)
  (bind _returnvalue_2 (`KismetArrayLibrary.Array_Add` (`self.Ants`) _returnvalue))
  (bind _output_get (set `TCCPlayerController.BuilderQtt` (+ (stale _output_get) 1) _aspl_ctrl_tcc))
  (bind _output_get_2 (set `TCCPlayerController.AntsQtt` (+ (stale _output_get_2) 1) _aspl_ctrl_tcc))
  (add `BaseCharacter.OnDiedDelegate` _returnvalue (delegate `OnDiedDelegate_Event_1`))
  (bind _index (`/Game/HUD/Wid_InGame.AddNewAnt` (`/Game/Blueprints/PlCtrl_TCC.InGameHud` _aspl_ctrl_tcc) _returnvalue))
  (`KismetArrayLibrary.Array_Set` (`self.WidgetIndex`) _returnvalue_2 _index true))

(event `OnDiedDelegate_Event_1`
  (params (DeadCharacter :type "BaseCharacter Object Reference"))
  (bind _ants (`self.Ants`))
  (bind _returnvalue (`KismetArrayLibrary.Array_Find` _ants DeadCharacter))
  (bind _aspl_ctrl_tcc (cast `/Game/Blueprints/PlCtrl_TCC` (`GameplayStatics.GetPlayerController` 0)))
  (bind _output_get (set `TCCPlayerController.BuilderQtt` (- (stale _output_get) 1) _aspl_ctrl_tcc))
  (bind _output_get_2 (set `TCCPlayerController.AntsQtt` (- (stale _output_get_2) 1) _aspl_ctrl_tcc))
  (`/Game/HUD/Wid_InGame.RemoveAnt` (`/Game/Blueprints/PlCtrl_TCC.InGameHud` _aspl_ctrl_tcc) _returnvalue)
  (`KismetArrayLibrary.Array_Remove` (`self.WidgetIndex`) _returnvalue)
  (`KismetArrayLibrary.Array_RemoveItem` _ants DeadCharacter)
  (bind _output_get_3 (set `TCCPlayerController.BuilderDead` (+ (stale _output_get_3) 1) _aspl_ctrl_tcc))
  (if (and (<= (`TCCPlayerController.AntsQtt` _aspl_ctrl_tcc) 0) (`self.CanGameOver`))
    (`/Game/Blueprints/PlCtrl_TCC.GameOver` _aspl_ctrl_tcc)))

(event `AddNewProcessor`
  (bind _aspl_ctrl_tcc (cast `/Game/Blueprints/PlCtrl_TCC` (`GameplayStatics.GetPlayerController` 0)))
  (bind _returnvalue (`|SpawnActorFromClass` "/Game/Blueprints/Characters/CharacterBlueprints/Ants/CharBP_Processor.CharBP_Processor_C" (`KismetMathLibrary.MakeTransform` (950.0 0.0 30.0)) "AlwaysSpawn" "OverrideRootScale"))
  (`Pawn.SpawnDefaultController` _returnvalue)
  (bind _returnvalue_2 (`KismetArrayLibrary.Array_Add` (`self.Ants`) _returnvalue))
  (bind _output_get (set `TCCPlayerController.ProcessorQtt` (+ (stale _output_get) 1) _aspl_ctrl_tcc))
  (bind _output_get_2 (set `TCCPlayerController.AntsQtt` (+ (stale _output_get_2) 1) _aspl_ctrl_tcc))
  (add `BaseCharacter.OnDiedDelegate` _returnvalue (delegate `OnDiedDelegate_Event_2`))
  (bind _index (`/Game/HUD/Wid_InGame.AddNewAnt` (`/Game/Blueprints/PlCtrl_TCC.InGameHud` _aspl_ctrl_tcc) _returnvalue))
  (`KismetArrayLibrary.Array_Set` (`self.WidgetIndex`) _returnvalue_2 _index true))

(event `OnDiedDelegate_Event_2`
  (params (DeadCharacter :type "BaseCharacter Object Reference"))
  (bind _ants (`self.Ants`))
  (bind _returnvalue (`KismetArrayLibrary.Array_Find` _ants DeadCharacter))
  (bind _aspl_ctrl_tcc (cast `/Game/Blueprints/PlCtrl_TCC` (`GameplayStatics.GetPlayerController` 0)))
  (bind _output_get (set `TCCPlayerController.ProcessorQtt` (- (stale _output_get) 1) _aspl_ctrl_tcc))
  (bind _output_get_2 (set `TCCPlayerController.AntsQtt` (- (stale _output_get_2) 1) _aspl_ctrl_tcc))
  (`/Game/HUD/Wid_InGame.RemoveAnt` (`/Game/Blueprints/PlCtrl_TCC.InGameHud` _aspl_ctrl_tcc) _returnvalue)
  (`KismetArrayLibrary.Array_Remove` (`self.WidgetIndex`) _returnvalue)
  (`KismetArrayLibrary.Array_RemoveItem` _ants DeadCharacter)
  (bind _output_get_3 (set `TCCPlayerController.ProcessorDead` (+ (stale _output_get_3) 1) _aspl_ctrl_tcc))
  (if (and (<= (`TCCPlayerController.AntsQtt` _aspl_ctrl_tcc) 0) (`self.CanGameOver`))
    (`/Game/Blueprints/PlCtrl_TCC.GameOver` _aspl_ctrl_tcc)))

(event `AddNewGuard`
  (bind _aspl_ctrl_tcc (cast `/Game/Blueprints/PlCtrl_TCC` (`GameplayStatics.GetPlayerController` 0)))
  (bind _returnvalue (`|SpawnActorFromClass` "/Game/Blueprints/Characters/CharacterBlueprints/Ants/CharBP_Guard.CharBP_Guard_C" (`KismetMathLibrary.MakeTransform` (950.0 0.0 30.0)) "AlwaysSpawn" "OverrideRootScale"))
  (`Pawn.SpawnDefaultController` _returnvalue)
  (bind _returnvalue_2 (`KismetArrayLibrary.Array_Add` (`self.Ants`) _returnvalue))
  (bind _output_get (set `TCCPlayerController.GuardQtt` (+ (stale _output_get) 1) _aspl_ctrl_tcc))
  (bind _output_get_2 (set `TCCPlayerController.AntsQtt` (+ (stale _output_get_2) 1) _aspl_ctrl_tcc))
  (add `BaseCharacter.OnDiedDelegate` _returnvalue (delegate `OnDiedDelegate_Event_3`))
  (bind _index (`/Game/HUD/Wid_InGame.AddNewAnt` (`/Game/Blueprints/PlCtrl_TCC.InGameHud` _aspl_ctrl_tcc) _returnvalue))
  (`KismetArrayLibrary.Array_Set` (`self.WidgetIndex`) _returnvalue_2 _index true))

(event `OnDiedDelegate_Event_3`
  (params (DeadCharacter :type "BaseCharacter Object Reference"))
  (bind _ants (`self.Ants`))
  (bind _returnvalue (`KismetArrayLibrary.Array_Find` _ants DeadCharacter))
  (bind _aspl_ctrl_tcc (cast `/Game/Blueprints/PlCtrl_TCC` (`GameplayStatics.GetPlayerController` 0)))
  (bind _output_get (set `TCCPlayerController.GuardQtt` (- (stale _output_get) 1) _aspl_ctrl_tcc))
  (bind _output_get_2 (set `TCCPlayerController.AntsQtt` (- (stale _output_get_2) 1) _aspl_ctrl_tcc))
  (`/Game/HUD/Wid_InGame.RemoveAnt` (`/Game/Blueprints/PlCtrl_TCC.InGameHud` _aspl_ctrl_tcc) _returnvalue)
  (`KismetArrayLibrary.Array_Remove` (`self.WidgetIndex`) _returnvalue)
  (`KismetArrayLibrary.Array_RemoveItem` _ants DeadCharacter)
  (bind _output_get_3 (set `TCCPlayerController.GuardDead` (+ (stale _output_get_3) 1) _aspl_ctrl_tcc))
  (if (and (<= (`TCCPlayerController.AntsQtt` _aspl_ctrl_tcc) 0) (`self.CanGameOver`))
    (`/Game/Blueprints/PlCtrl_TCC.GameOver` _aspl_ctrl_tcc)))

(event `AddNewCleaner`
  (bind _aspl_ctrl_tcc (cast `/Game/Blueprints/PlCtrl_TCC` (`GameplayStatics.GetPlayerController` 0)))
  (bind _returnvalue (`|SpawnActorFromClass` "/Game/Blueprints/Characters/CharacterBlueprints/Ants/CharBP_Cleaner.CharBP_Cleaner_C" (`KismetMathLibrary.MakeTransform` (950.0 0.0 30.0)) "AlwaysSpawn" "OverrideRootScale"))
  (`Pawn.SpawnDefaultController` _returnvalue)
  (bind _returnvalue_2 (`KismetArrayLibrary.Array_Add` (`self.Ants`) _returnvalue))
  (bind _output_get (set `TCCPlayerController.CleanerQtt` (+ (stale _output_get) 1) _aspl_ctrl_tcc))
  (bind _output_get_2 (set `TCCPlayerController.AntsQtt` (+ (stale _output_get_2) 1) _aspl_ctrl_tcc))
  (add `BaseCharacter.OnDiedDelegate` _returnvalue (delegate `OnDiedDelegate_Event_4`))
  (bind _index (`/Game/HUD/Wid_InGame.AddNewAnt` (`/Game/Blueprints/PlCtrl_TCC.InGameHud` _aspl_ctrl_tcc) _returnvalue))
  (`KismetArrayLibrary.Array_Set` (`self.WidgetIndex`) _returnvalue_2 _index true))

(event `OnDiedDelegate_Event_4`
  (params (DeadCharacter :type "BaseCharacter Object Reference"))
  (bind _ants (`self.Ants`))
  (bind _returnvalue (`KismetArrayLibrary.Array_Find` _ants DeadCharacter))
  (bind _aspl_ctrl_tcc (cast `/Game/Blueprints/PlCtrl_TCC` (`GameplayStatics.GetPlayerController` 0)))
  (bind _output_get (set `TCCPlayerController.CleanerQtt` (- (stale _output_get) 1) _aspl_ctrl_tcc))
  (bind _output_get_2 (set `TCCPlayerController.AntsQtt` (- (stale _output_get_2) 1) _aspl_ctrl_tcc))
  (`/Game/HUD/Wid_InGame.RemoveAnt` (`/Game/Blueprints/PlCtrl_TCC.InGameHud` _aspl_ctrl_tcc) _returnvalue)
  (`KismetArrayLibrary.Array_Remove` (`self.WidgetIndex`) _returnvalue)
  (`KismetArrayLibrary.Array_RemoveItem` _ants DeadCharacter)
  (bind _output_get_3 (set `TCCPlayerController.CleanerDead` (+ (stale _output_get_3) 1) _aspl_ctrl_tcc))
  (if (and (<= (`TCCPlayerController.AntsQtt` _aspl_ctrl_tcc) 0) (`self.CanGameOver`))
    (`/Game/Blueprints/PlCtrl_TCC.GameOver` _aspl_ctrl_tcc)))

(event `Retreat`
  (bind _ants (`self.Ants`))
  (for _array_element _ants
    (`BaseCharacter.Retreat` _array_element))
  (`KismetSystemLibrary.Delay` 7.0)
  (for _array_element_2 _ants
    (bind _returnvalue (`AIBlueprintHelperLibrary.GetAIController` _array_element_2))
    (bind _asaictrl_cleaner (cast `AICtrl_Cleaner` _returnvalue)
      (:`then`
        (`AICtrl_Cleaner.SetUnderAttack` _asaictrl_cleaner false))
      (:`CastFailed`
        (bind _asaictrl_builder (cast `AICtrl_Builder` _returnvalue)
          (:`then`
            (`AICtrl_Builder.SetUnderAttack` _asaictrl_builder false))
          (:`CastFailed`
            (bind _asaictrl_collector (cast `AICtrl_Collector` _returnvalue)
              (:`then`
                (`AICtrl_Collector.SetUnderAttack` _asaictrl_collector false))
              (:`CastFailed`
                (bind _asaictrl_guard (cast `AICtrl_Guard` _returnvalue)
                  (:`then`
                    (`AICtrl_Guard.SetUnderAttack` _asaictrl_guard false))
                  (:`CastFailed`
                    (bind _asaictrl_processor (cast `AICtrl_Processor` _returnvalue)
                      (:`then`
                        (`AICtrl_Processor.SetUnderAttack` _asaictrl_processor false))
                      (:`CastFailed`
                        _))))))))))
    (bind _aspl_ctrl_tcc (cast `/Game/Blueprints/PlCtrl_TCC` (`GameplayStatics.GetPlayerController` 0)))
    (set `TCCPlayerController.EnemiesLeft` 0 _aspl_ctrl_tcc)))

(fn `UserConstructionScript`)