(event `self.ReceiveBeginPlay`
  (bind _returnvalue (`|CreateWidget` "/Game/HUD/Wid_Menu.Wid_Menu_C"))
  (set `self.Menu` _returnvalue)
  (bind _returnvalue_2 (`|CreateWidget` "/Game/HUD/Wid_InGame.Wid_InGame_C"))
  (set `self.InGameHud` _returnvalue_2)
  (bind _returnvalue_3 (`|CreateWidget` "/Game/HUD/Wid_PauseMenu.Wid_PauseMenu_C"))
  (set `self.PauseMenu` _returnvalue_3)
  (set `PlayerController.bShowMouseCursor` true)
  (`self.StartMenu`))

(event `StartGame`
  (params (Level :type Integer))
  (bind _ingamehud (`self.InGameHud`))
  (bind _menu (`self.Menu`))
  (bind _pausemenu (`self.PauseMenu`))
  (`/Engine/EditorBlueprintResources/StandardMacros.IsValid` _menu
    (:`Is Valid`
      (`Widget.RemoveFromParent` _menu))
    (:`Is Not Valid`
      _))
  (`/Engine/EditorBlueprintResources/StandardMacros.IsValid` _ingamehud
    (:`Is Valid`
      _)
    (:`Is Not Valid`
      (bind _returnvalue (`|CreateWidget` "/Game/HUD/Wid_InGame.Wid_InGame_C"))
      (set `self.InGameHud` _returnvalue)))
  (`UserWidget.AddToViewport` _ingamehud 0)
  (`/Engine/EditorBlueprintResources/StandardMacros.IsValid` _pausemenu
    (:`Is Valid`
      (`Widget.RemoveFromParent` _pausemenu))
    (:`Is Not Valid`
      _))
  (`GameplayStatics.SetGamePaused` false)
  (`self.GameStarted` Level))

(event `StartMenu`
  (bind _menu (`self.Menu`))
  (bind _pausemenu (`self.PauseMenu`))
  (bind _ingamehud (`self.InGameHud`))
  (`/Engine/EditorBlueprintResources/StandardMacros.IsValid` _menu
    (:`Is Valid`
      _)
    (:`Is Not Valid`
      (bind _returnvalue (`|CreateWidget` "/Game/HUD/Wid_Menu.Wid_Menu_C"))
      (set `self.Menu` _returnvalue)))
  (`UserWidget.AddToViewport` _menu 0)
  (`/Engine/EditorBlueprintResources/StandardMacros.IsValid` _ingamehud
    (:`Is Valid`
      (`Widget.RemoveFromParent` _ingamehud)
      (`/Engine/EditorBlueprintResources/StandardMacros.IsValid` _pausemenu
        (:`Is Valid`
          (`Widget.RemoveFromParent` _pausemenu))
        (:`Is Not Valid`
          _))
      (`GameplayStatics.SetGamePaused` true))))

(event `PauseGame`
  (bind _menu (`self.Menu`))
  (bind _ingamehud (`self.InGameHud`))
  (bind _pausemenu (`self.PauseMenu`))
  (`/Engine/EditorBlueprintResources/StandardMacros.IsValid` _menu
    (:`Is Valid`
      (`Widget.RemoveFromParent` _menu))
    (:`Is Not Valid`
      _))
  (`/Engine/EditorBlueprintResources/StandardMacros.IsValid` _ingamehud
    (:`Is Valid`
      (`Widget.RemoveFromParent` _ingamehud))
    (:`Is Not Valid`
      _))
  (`/Engine/EditorBlueprintResources/StandardMacros.IsValid` _pausemenu
    (:`Is Valid`
      _)
    (:`Is Not Valid`
      (bind _returnvalue (`|CreateWidget` "/Game/HUD/Wid_PauseMenu.Wid_PauseMenu_C"))
      (set `self.PauseMenu` _returnvalue)))
  (`UserWidget.AddToViewport` _pausemenu 0)
  (`GameplayStatics.SetGamePaused` true))

(event `ContinueGame`
  (bind _pausemenu (`self.PauseMenu`))
  (bind _ingamehud (`self.InGameHud`))
  (bind _menu (`self.Menu`))
  (`/Engine/EditorBlueprintResources/StandardMacros.IsValid` _menu
    (:`Is Valid`
      (`Widget.RemoveFromParent` _menu))
    (:`Is Not Valid`
      _))
  (`/Engine/EditorBlueprintResources/StandardMacros.IsValid` _ingamehud
    (:`Is Valid`
      _)
    (:`Is Not Valid`
      (bind _returnvalue (`|CreateWidget` "/Game/HUD/Wid_InGame.Wid_InGame_C"))
      (set `self.InGameHud` _returnvalue)))
  (`UserWidget.AddToViewport` _ingamehud 0)
  (`/Engine/EditorBlueprintResources/StandardMacros.IsValid` _pausemenu
    (:`Is Valid`
      (`Widget.RemoveFromParent` _pausemenu))
    (:`Is Not Valid`
      _))
  (`GameplayStatics.SetGamePaused` false))

(event `GameOver`
  (bind _menu (`self.Menu`))
  (bind _ingamehud (`self.InGameHud`))
  (bind _pausemenu (`self.PauseMenu`))
  (`/Engine/EditorBlueprintResources/StandardMacros.IsValid` _menu
    (:`Is Valid`
      (`Widget.RemoveFromParent` _menu))
    (:`Is Not Valid`
      _))
  (`/Engine/EditorBlueprintResources/StandardMacros.IsValid` _ingamehud
    (:`Is Valid`
      (`Widget.RemoveFromParent` _ingamehud))
    (:`Is Not Valid`
      _))
  (`/Engine/EditorBlueprintResources/StandardMacros.IsValid` _pausemenu
    (:`Is Valid`
      (`Widget.RemoveFromParent` _pausemenu))
    (:`Is Not Valid`
      _))
  (bind _returnvalue (`|CreateWidget` "/Game/HUD/Wid_GameOver.Wid_GameOver_C" null "Game Over"))
  (`UserWidget.AddToViewport` _returnvalue 0)
  (`GameplayStatics.SetGamePaused` true))

(event `YouWin`
  (bind _ingamehud (`self.InGameHud`))
  (bind _pausemenu (`self.PauseMenu`))
  (bind _menu (`self.Menu`))
  (`/Engine/EditorBlueprintResources/StandardMacros.IsValid` _menu
    (:`Is Valid`
      (`Widget.RemoveFromParent` _menu))
    (:`Is Not Valid`
      _))
  (`/Engine/EditorBlueprintResources/StandardMacros.IsValid` _ingamehud
    (:`Is Valid`
      (`Widget.RemoveFromParent` _ingamehud))
    (:`Is Not Valid`
      _))
  (`/Engine/EditorBlueprintResources/StandardMacros.IsValid` _pausemenu
    (:`Is Valid`
      (`Widget.RemoveFromParent` _pausemenu))
    (:`Is Not Valid`
      _))
  (bind _returnvalue (`|CreateWidget` "/Game/HUD/Wid_GameOver.Wid_GameOver_C" null "You Win"))
  (`UserWidget.AddToViewport` _returnvalue 0)
  (`GameplayStatics.SetGamePaused` true))

(fn `UserConstructionScript`)