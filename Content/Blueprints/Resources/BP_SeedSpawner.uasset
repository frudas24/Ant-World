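; BP_SeedSpawner spawns BP_Seed actors at random navigable points around a set of Locations.
; SpawnSeeds, not called from BeginPlay, reads AntsQtt from PlCtrl_TCC and spawns that many seeds, each near a randomly picked location.
; The spawn loop also triggers a delayed re-call of SpawnSeeds, so spawning repeats at the supplied interval.
; Disconnected alternative spawn logic remains but never runs.
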(event `self.ReceiveBeginPlay`)

(event `self.ReceiveActorBeginOverlap`
  (params (OtherActor :type "Actor Object Reference")))

(event `self.ReceiveTick`
  (params (DeltaSeconds :type "Float (single-precision)")))

(event `SpawnSeeds`
  (params (Delay :type "Float (double-precision)"))
  (bind _locations (`self.Locations`))
  (`KismetSystemLibrary.Delay` 0.5)
  (bind _aspl_ctrl_tcc (cast `/Game/Blueprints/PlCtrl_TCC` (`GameplayStatics.GetPlayerController` 0)))
  (for _ (range (`TCCPlayerController.AntsQtt` _aspl_ctrl_tcc))
    (`|SpawnActorFromClass` "/Game/Blueprints/Resources/BP_Seed.BP_Seed_C" (`KismetMathLibrary.MakeTransform` (`NavigationSystem.GetRandomPointInNavigableRadius` (`KismetArrayLibrary.Array_Get` _locations (`KismetMathLibrary.RandomIntegerInRange` 0 (- (`KismetArrayLibrary.Array_Length` _locations) 1))) 350.0)) "AlwaysSpawn" "OverrideRootScale")
    ;[1 1 1] Default is 200
    (`KismetSystemLibrary.Delay` Delay) ; Default is 200
    (`self.SpawnSeeds` Delay)))

(fn `UserConstructionScript`)